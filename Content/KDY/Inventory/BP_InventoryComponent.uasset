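; BP_InventoryComponent is a component that creates and opens the player's inventory UI.
; On BeginPlay it creates WBP_Inventory, adds it to the viewport and hides it as Collapsed.
; The IA_Inventory input shows the collapsed widget with keyboard focus, switches to UI-only input with a mouse cursor and plays its opening animation.
; It only opens the inventory, with no closing logic in this graph.
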(event Input|EnhancedActionEvents|EnhancedInputActionIA_Inventory
  (params (ActionValue :type Boolean) (ElapsedSeconds :type Float%20%28double-precision%29) (TriggeredSeconds :type Float%20%28double-precision%29) (InputAction :type Input%20Action%20Object%20Reference :default "/Game/ThirdPerson/Input/Actions/IA_Inventory.IA_Inventory"))
  (bind _returnvalue (Game|GetPlayerController 0))
  (bind _inventorywidget (Variables|Default|GetInventoryWidget))
  (bind _inventorywidget_2 (Variables|Default|GetInventoryWidget))
  ;[0.15 0.15 0.15 0.5] 인벤토리 열기
  (:Started
    (if (Utilities|Enum|Equal(Enum) (Widget|GetVisibility (Variables|Default|GetInventoryWidget)) "Collapsed")
      (Widget|SetVisibility _inventorywidget "Visible")
      (Widget|SetKeyboardFocus _inventorywidget)
      (Input|SetInputModeUIOnly _returnvalue 0 "DoNotLock" true)
      (Variables|/Script/Engine.PlayerController|SetbShowMouseCursor _returnvalue true)
      (UserInterface|Animation|PlayAnimation _inventorywidget_2 (Variables|/Game/KDY/Inventory/WBP_Inventory.WBP_Inventory_C|GetInventoryAnimation _inventorywidget_2) 0.0 1 "Forward" 1.0 false))))

(event EventBeginPlay
  (bind _returnvalue (UserInterface|CreateWidget "/Game/KDY/Inventory/WBP_Inventory.WBP_Inventory_C"))
  (bind _output_get (Variables|Default|SetInventoryWidget _returnvalue))
  (UserInterface|Viewport|AddtoViewport _output_get 0)
  (Widget|SetVisibility (Variables|Default|GetInventoryWidget) "Collapsed"))

(event EventTick
  (params (DeltaSeconds :type Float%20%28single-precision%29)))