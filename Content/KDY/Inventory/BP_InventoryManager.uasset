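; BP_InventoryManager creates and manages the player's inventory UI and requests item additions and removals.
; On BeginPlay it creates a collapsed WBP_Inventory, binds its window to itself and calls UpdateInventoryData.
; OpenInventory reveals the widget with animations, UI-only input and a mouse cursor.
; A test loop randomly adds and subtracts items every two seconds; the subtraction log rolls its ID separately from the one used.
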(event Custom|OpenInventory
  (bind _returnvalue (Game|GetPlayerController 0))
  (bind _inventorywidget (Variables|Default|GetInventoryWidget))
  (bind _inventorywidget_2 (Variables|Default|GetInventoryWidget))
  ;[0.15 0.15 0.15 0.5] 인벤토리 열기
  (if (Utilities|Enum|Equal(Enum) (Widget|GetVisibility (Variables|Default|GetInventoryWidget)) "Collapsed")
    (Widget|SetVisibility _inventorywidget_2 "Visible")
    (Widget|SetKeyboardFocus _inventorywidget_2)
    (Input|SetInputModeUIOnly _returnvalue 0 "DoNotLock" true)
    (Variables|/Script/Engine.PlayerController|SetbShowMouseCursor _returnvalue true)
    (UserInterface|Animation|PlayAnimation _inventorywidget (Variables|/Game/KDY/Inventory/WBP_Inventory.WBP_Inventory_C|GetInventoryAnimation _inventorywidget) 0.0 1 "Forward" 1.0 false)
    (UserInterface|Animation|PlayAnimation _inventorywidget (Variables|/Game/KDY/Inventory/WBP_Inventory.WBP_Inventory_C|GetItemPopUpAnimation _inventorywidget) 0.0 1 "Forward" 1.0 false)))

(event EventBeginPlay
  (Utilities|FlowControl|Sequence
    (:then_0
      (bind _returnvalue (UserInterface|CreateWidget "/Game/KDY/Inventory/WBP_Inventory.WBP_Inventory_C"))
      (bind _output_get (Variables|Default|SetInventoryWidget _returnvalue))
      (Utilities|FlowControl|Sequence
        (:then_0
          (UserInterface|Viewport|AddtoViewport _output_get 0)
          (Widget|SetVisibility _output_get "Collapsed"))
        (:then_1
          (bind _output_get_2 (Variables|Default|SetInventoryWindowWidget (Variables|/Game/KDY/Inventory/WBP_Inventory.WBP_Inventory_C|GetWBP_InventoryWindow _output_get)))
          (bind _aswbp_inventory_window (Utilities|Casting|CastToWBP_InventoryWindow _output_get_2))
          (Default|BindwithManager _aswbp_inventory_window self))))
    (:then_1
      (Class|InventoryManager|UpdateInventoryData)
      ;[0.15 0.15 0.15 0.5] Test
      (CallFunction|AddItemEvent :!label _label)
      (CallFunction|SubtractItemEvent)
      (Utilities|FlowControl|Delay 2.0)
      (goto _label))))

(event Custom|AddItemEvent
  (bind _output_get (Variables|Default|SetTestAddID (Math|Random|RandomInteger 2)))
  (bind _returnvalue (Class|InventoryManager|TryAddItem _output_get 2))
  (if _returnvalue
    (Development|PrintString (Utilities|String|Append "Success Add Item : " (Utilities|String|ToString(Integer) (Variables|Default|GetTestAddID)) ", Count: 2"))))

(event Custom|SubtractItemEvent
  (bind _returnvalue (Math|Random|RandomInteger 2))
  (Variables|Default|SetTestSubID _returnvalue)
  (bind _returnvalue_2 (Class|InventoryManager|TrySubtractItem _returnvalue 1))
  (if _returnvalue_2
    (Development|PrintString (Utilities|String|Append "Try Sub Item : " (Utilities|String|ToString(Integer) (Variables|Default|GetTestSubID)) ", Count: 1"))))

(fn ConstructionScript)