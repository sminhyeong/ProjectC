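; BP_ChestComponent is an interaction component for reward chests that responds when a dungeon character interacts with its target actor.
; ResInteract casts the interactor and its controller, asks BP_PlayerController to create the reward widget, then hides the target actor in game.
; HasInteraction always returns false.
; NewFunction is empty, and the local widget, fade-in and input-mode nodes in both graphs are unconnected leftovers.
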(event EventResInteract
  (params (Interactor :type Actor%20Object%20Reference) (TargetActor :type Actor%20Object%20Reference))
  (bind _asbp_dungeon_character (Utilities|Casting|CastToBP_DungeonCharacter Interactor))
  (bind _asbp_player_controller (Utilities|Casting|CastToBP_PlayerController (Pawn|GetController _asbp_dungeon_character)))
  (Default|CreateRewardWidget _asbp_player_controller)
  (Rendering|SetActorHiddenInGame TargetActor true))

(fn HasInteraction
  (params (Interactor :type Actor%20Object%20Reference) (TargetActor :type Actor%20Object%20Reference))
  (return false))

(fn NewFunction)