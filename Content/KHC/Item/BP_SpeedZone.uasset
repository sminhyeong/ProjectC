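; BP_SpeedZone is a zone actor that changes the player's walk speed and sets off a staggered sequence of fires.
; On box overlap by BP_Player, it applies its MaxWalkSpeed and starts a looping timer on SetFire.
; SetFire starts the next Fire array entry each tick, stopping after the fifth; the index never resets.
; Leaving the box sets walk speed to a hard-coded value without stopping the timer.
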(event OnComponentBeginOverlap(Box)
  (params (OverlappedComponent :type Primitive%20Component%20Object%20Reference) (OtherActor :type Actor%20Object%20Reference) (OtherComp :type Primitive%20Component%20Object%20Reference) (OtherBodyIndex :type Integer) (bFromSweep :type Boolean) (SweepResult :type Hit%20Result%20Structure%20%28by%20ref%29))
  (bind _asbp_player (Utilities|Casting|CastToBP_Player OtherActor))
  (Variables|/Script/Engine.CharacterMovementComponent|SetMaxWalkSpeed (Variables|/Script/Engine.Character|GetCharacterMovement _asbp_player) (Variables|Default|GetMax%20Walk%20Speed))
  (Utilities|Time|SetTimerbyFunctionName 0 "SetFire" 0.3 true))

(event OnComponentEndOverlap(Box)
  (params (OverlappedComponent :type Primitive%20Component%20Object%20Reference) (OtherActor :type Actor%20Object%20Reference) (OtherComp :type Primitive%20Component%20Object%20Reference) (OtherBodyIndex :type Integer))
  (bind _asbp_player (Utilities|Casting|CastToBP_Player OtherActor))
  (Variables|/Script/Engine.CharacterMovementComponent|SetMaxWalkSpeed (Variables|/Script/Engine.Character|GetCharacterMovement _asbp_player) 5e+02))

(event EventBeginPlay)

(event Collision|EventActorBeginOverlap
  (params (OtherActor :type Actor%20Object%20Reference)))

(event EventTick
  (params (DeltaSeconds :type Float%20%28single-precision%29)))

(fn ConstructionScript)

(fn SetFire
  (Default|StartFire (Utilities|Array|Get(acopy) (Variables|Default|GetFire) (Variables|Default|GetFireIndex)))
  (bind _output_get (Variables|Default|SetFireIndex (+ (Variables|Default|GetFireIndex) 1)))
  (Development|PrintString (Utilities|String|ToString(Integer) _output_get))
  (if (== _output_get 5)
    (Utilities|Time|ClearTimerbyFunctionName 0 "SetFire")))