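; BP_BossAICon is the boss AI controller, which sets team ID 1 and runs the BT_BossState behavior tree on BeginPlay.
; On authority, a perceived BP_Player is written to the blackboard and the AIState key is set.
; A looping timer polls that key and forwards changes through CallEVUpdateAIStates.
; It also binds a perception-updated delegate; EV_TargerUpdated only prints the first actor's name.
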(event OnTargetPerceptionUpdated(AIPerception)
  (params (Actor :type Actor%20Object%20Reference) (Stimulus :type AI%20Stimulus%20Structure))
  (Networking|SwitchHasAuthority
    (:Authority
      (bind _asbp_player (Utilities|Casting|CastToBP_Player Actor))
      (AI|Components|Blackboard|SetValueasObject (AI|GetBlackboard 0) (Utilities|Name|MakeLiteralName "Player") _asbp_player)
      (AI|Components|Blackboard|SetValueasEnum (AI|GetBlackboard 0) (Utilities|Name|MakeLiteralName "AIState") (Utilities|Enum|LiteralenumEN_AIState "NewEnumerator4")))))

(event EventBeginPlay
  (Utilities|Struct|SetmembersinGenericTeamId (Utilities|Struct|MakeGenericTeamId 1))
  ;[0.15 0.15 0.15 0.5] OK
  (AI|RunBehaviorTree "/Game/KJK/GM/AI/BOSSAI/BT_BossState.BT_BossState")
  (Utilities|Time|SetTimerbyFunctionName 0 "UpdateAIState" 0.01 true)
  (EventDispatchers|BindEventtoOnPerceptionUpdated (Variables|Default|GetAIPerception) (EventDispatchers|CreateEvent :!event EVTargerUpdated)))

(fn ConstructionScript)

(fn UpdateAIState
  (bind _returnvalue (AI|GetBlackboard 0))
  (bind _returnvalue_2 (Utilities|Name|MakeLiteralName "AIState"))
  (bind _returnvalue_3 (Class|BlackboardComponent|GetValueasEnum _returnvalue _returnvalue_2))
  (bind _returnvalue_4 (Utilities|Enum|ByteToEnumEN_AIState _returnvalue_3))
  (if (not (Utilities|Enum|Equal(Enum) _returnvalue_4 (Variables|Default|GetAIState)))
    (bind _output_get (Variables|Default|SetAIState _returnvalue_4))
    (Default|CallEVUpdateAIStates _output_get)))

(fn EVTargerUpdated
  (params (UpdatedActors :type Array%20of%20Actor%20Object%20References))
  (Development|PrintString (Utilities|GetDisplayName (Utilities|Array|Get(acopy) UpdatedActors)))
  (return))