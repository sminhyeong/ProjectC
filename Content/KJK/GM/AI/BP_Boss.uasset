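; Boss AI character that extends its parent with player detection, a boss health display and a death notification to the game state.
; On authority, every tick passes sight-perceived players to their AIPercept.
; On spawn and state changes, it pushes HP to the first player's pawn via ResBossHP.
; PlayerDeathReq calls the game state's MonsterDeathReq; DoDeath only adds a debug print, as chest and portal spawning is disconnected.
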(event Custom|ReqPerception
  (Networking|SwitchHasAuthority
    (:Authority
      (for _array_element (Class|AIPerceptionComponent|GetCurrentlyPerceivedActors (Class|AIController|GetAIPerceptionComponent (AI|GetAIController self)) "/Script/AIModule.AISense_Sight")
        (bind _asbp_player (Utilities|Casting|CastToBP_Player _array_element))
        (Default|AIPercept _asbp_player _asbp_player)))))

(event Custom|ReqHPWidget
  (bind _characterstate (Variables|Default|GetCharacterState))
  (bind _asbp_player (Utilities|Casting|CastToBP_Player (Pawn|GetControlledPawn (Game|GetPlayerController 0))))
  (EventDispatchers|AssignDSChangeStates (EventDispatchers|CreateEvent :!event BPBossAutoGenFunc))
  (Utilities|FlowControl|Delay 1.0)
  (Default|ResBossHP _asbp_player (Variables|/Script/ProjectC.CharacterStateComponent|GetCurHP _characterstate) 0.0 0.0 (Variables|/Script/ProjectC.CharacterStateComponent|GetMaxHP _characterstate) 0.0 0.0))

(event EventBeginPlay
  (|CallParentFunction)
  (CallFunction|ReqHPWidget))

(event Collision|EventActorBeginOverlap
  (params (OtherActor :type Actor%20Object%20Reference))
  (|CallParentFunction OtherActor))

(event EventTick
  (params (DeltaSeconds :type Float%20%28single-precision%29))
  (|CallParentFunction DeltaSeconds)
  (CallFunction|ReqPerception))

(event EventDoDeath
  (|CallParentFunction)
  (Development|PrintString "spawn" true true "(R=0.000000,G=0.660000,B=1.000000,A=1.000000)" 1e+01))

(event EventPlayerDeathReq
  (|CallParentFunction)
  (bind _asbp_game_start_game_state (Utilities|Casting|CastToBP_GameStartGameState (Game|GetGameState)))
  (Default|MonsterDeathReq _asbp_game_start_game_state))

(fn ConstructionScript
  (|CallParentFunction))

(fn BPBossAutoGenFunc
  (params (CurHP :type Float%20%28double-precision%29) (CurShield :type Float%20%28double-precision%29) (CurMP :type Float%20%28double-precision%29) (MaxHP :type Float%20%28double-precision%29) (MaxShield :type Float%20%28double-precision%29) (MaxMP :type Float%20%28double-precision%29))
  (bind _asbp_player (Utilities|Casting|CastToBP_Player (Pawn|GetControlledPawn (Game|GetPlayerController 0))))
  (Default|ResBossHP _asbp_player CurHP 0.0 0.0 MaxHP 0.0 0.0))