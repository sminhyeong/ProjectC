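; BP_Monster is an AI monster that plays a randomly chosen skill animation while in the Attack state.
; On possession it binds to BP_AICon's AI state update event, and Tick dispatches on the stored AiState.
; BattleTick picks a random DT_SkillTest row and plays its montage.
; An IsPlayingSkill flag blocks further picks once set, and nothing in this file clears it.
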(event EventBeginPlay
  (|CallParentFunction))

(event Collision|EventActorBeginOverlap
  (params (OtherActor :type Actor%20Object%20Reference)))

(event EventTick
  (params (DeltaSeconds :type Float%20%28single-precision%29))
  (CallFunction|AITick))

(event EventPossessed
  (params (NewController :type Controller%20Object%20Reference))
  (CallFunction|InitAi NewController))

(fn ConstructionScript
  (|CallParentFunction))

(fn UpdateAIState
  (params (AiState :type EN_AIState%20Enum :default "NewEnumerator0"))
  (Variables|Default|SetAiState AiState))

(fn InitAi
  (params (AI :type Object%20Object%20Reference))
  (bind _asbp_aicon (Utilities|Casting|CastToBP_AICon AI))
  (EventDispatchers|BindEventtoEVUpdateAIStates _asbp_aicon (EventDispatchers|CreateEvent :!event UpdateAIState)))

(fn AITick
  (switch Utilities|FlowControl|Switch|SwitchonEN_AIState (Variables|Default|GetAiState)
    (:NewEnumerator2
      (CallFunction|BattleTick))))

(fn BattleTick
  ;[0.15 0.15 0.15 0.5] AIstructure 구조체를 기반으로 하는 데이터 테이블(목록)에서 랜덤으로 이름을 가져와서 그 이름에 해당하는 구조체의 애니메이션 실행
  ;;[0.15 0.15 0.15 0.5] 예외처리- 플레이 아닐시 발생
  (if (not (Variables|Default|GetisPlayingSkill))
    ;;[0.15 0.15 0.15 0.5] 데이터 테이블DT skill 가져오기
    (bind _outrownames (DataTable|GetDataTableRowNames 0))
    ;;[0.15 0.15 0.15 0.5] DT SKill에서 이름배열 랜덤으로 가져오기-
    (bind _returnvalue (Utilities|GetDataTableRow "/Game/KJK/GM/DT_SkillTest.DT_SkillTest" (.OutItem (Utilities|Array|Random _outrownames)))
      (:then
        ;;[0.15 0.15 0.15 0.5] AIstructure의 애니 실행
        (Animation|PlayAnimMontage (.Animation (Utilities|Struct|BreakST_SkillTest _returnvalue)) 1.0 "None")
        (Variables|Default|SetisPlayingSkill true)))))