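; BP_BattleManager is a battle manager that holds damage, shield, heal and MP-use amounts.
; Its Cal functions store and return their inputs unchanged, with no formulas applied yet.
; RepNotify functions on those four variables broadcast matching event dispatchers with the new values.
; SetAdditionalStats, intended for stat bonuses from equipped items, is a stub that only casts the game instance.
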(event EventBeginPlay)

(event Collision|EventActorBeginOverlap
  (params (OtherActor :type Actor%20Object%20Reference)))

(event EventTick
  (params (DeltaSeconds :type Float%20%28single-precision%29)))

(fn ConstructionScript)

(fn CalDamage
  (params (BaseDamage :type Float%20%28single-precision%29))
  (bind _output_get (Variables|Default|SetDamageAmount BaseDamage))
  (return _output_get))

(fn CalShield
  (params (ShieldAmount :type Float%20%28double-precision%29))
  (bind _output_get (Variables|Default|SetShieldAmount ShieldAmount))
  (return _output_get))

(fn CalHeal
  (params (HealAmount :type Float%20%28double-precision%29))
  (bind _output_get (Variables|Default|SetHealAmount HealAmount))
  (return _output_get))

(fn CalMP
  (params (MPUseAmount :type Float%20%28double-precision%29))
  (bind _output_get (Variables|Default|SetMPUseAmount MPUseAmount))
  (return _output_get))

(fn SetAdditionalStats
  ;[0.15 0.15 0.15 0.5] 아이템 착용시 추가 스탯
  (bind _asbp_game_instance (Utilities|Casting|CastToBP_GameInstance (Game|GetGameInstance))))

(fn OnRepDamageAmount
  (Default|CallDSDamageAmount (Variables|Default|GetDamageAmount)))

(fn OnRepHealAmount
  (Default|CallDSHealAmount (Variables|Default|GetHealAmount)))

(fn OnRepShieldAmount
  (Default|CallDSShieldAmount (Variables|Default|GetShieldAmount)))

(fn OnRepMPUseAmount
  (Default|CallDSMPUseAmount (Variables|Default|GetMPUseAmount)))