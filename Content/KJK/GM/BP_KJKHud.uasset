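; BP_KJKHud is a HUD Blueprint that creates the battle widget on BeginPlay and displays the player's HP, MP and shield.
; BindPlayerState binds to BP_Player's state-change dispatcher and pushes initial values, retrying on a very short timer until the controlled pawn casts successfully.
; EVChangeState passes current values to BattleWidget, reading maximums from the controlled BP_BaseCharacter's CharacterState.
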(event EventBeginPlay
  (bind _returnvalue (UserInterface|CreateWidget "/Game/KJK/Widget/BattleWidget.BattleWidget_C"))
  (bind _output_get (Variables|Default|SetBattleWidget _returnvalue))
  (UserInterface|Viewport|AddtoViewport _output_get 0)
  (CallFunction|BindPlayerState))

(event Collision|EventActorBeginOverlap
  (params (OtherActor :type Actor%20Object%20Reference)))

(event EventTick
  (params (DeltaSeconds :type Float%20%28single-precision%29)))

(fn ConstructionScript)

(fn BindPlayerState
  (bind _asbp_player (Utilities|Casting|CastToBP_Player (Pawn|GetControlledPawn (Game|GetPlayerController 0)))
    (:then
      (EventDispatchers|BindEventtoDSChangeStates _asbp_player (EventDispatchers|CreateEvent :!event EVChangeState))
      (CallFunction|EVChangeState (Variables|/Script/ProjectC.CharacterStateComponent|GetCurHP (Variables|/Game/KJK/GM/BP_BaseCharacter.BP_BaseCharacter_C|GetCharacterState _asbp_player)) (Variables|/Script/ProjectC.CharacterStateComponent|GetCurShield (Variables|/Game/KJK/GM/BP_BaseCharacter.BP_BaseCharacter_C|GetCharacterState _asbp_player)) (Variables|/Script/ProjectC.CharacterStateComponent|GetCurMP (Variables|/Game/KJK/GM/BP_BaseCharacter.BP_BaseCharacter_C|GetCharacterState _asbp_player))))
    (:CastFailed
      (Utilities|Time|SetTimerbyFunctionName 0 "BindPlayerState" 0.001))))

(fn EVChangeState
  (params (CurHP :type Float%20%28double-precision%29) (CurShield :type Float%20%28double-precision%29) (CurMP :type Float%20%28double-precision%29))
  (bind _battlewidget (Variables|Default|GetBattleWidget))
  (bind _asbp_base_character (Utilities|Casting|CastToBP_BaseCharacter (Pawn|GetControlledPawn (Game|GetPlayerController 0))))
  (Default|SetHP _battlewidget CurHP (Variables|/Script/ProjectC.CharacterStateComponent|GetMaxHP (Variables|/Game/KJK/GM/BP_BaseCharacter.BP_BaseCharacter_C|GetCharacterState _asbp_base_character)))
  (Default|SetMP _battlewidget CurMP (Variables|/Script/ProjectC.CharacterStateComponent|GetMaxMP (Variables|/Game/KJK/GM/BP_BaseCharacter.BP_BaseCharacter_C|GetCharacterState _asbp_base_character)))
  (Default|SetShield _battlewidget CurShield (Variables|/Script/ProjectC.CharacterStateComponent|GetMaxShield (Variables|/Game/KJK/GM/BP_BaseCharacter.BP_BaseCharacter_C|GetCharacterState _asbp_base_character))))