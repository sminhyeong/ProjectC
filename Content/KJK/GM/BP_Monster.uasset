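; BP_Monster is a monster Blueprint that passes perceived targets to its AI Blackboard.
; When AIPerception updates a target, it prints the actor's name and sensed flag for debugging.
; It then writes that actor to the "Player" key, whether sensing succeeded or not and without checking that it is a player.
; EV_UpdateAIState is an empty stub, and the default events are inactive.
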(event OnTargetPerceptionUpdated(AIPerception)
  (params (Actor :type Actor%20Object%20Reference) (Stimulus :type AI%20Stimulus%20Structure))
  (Development|PrintString (Utilities|String|Append "Target" (Utilities|GetDisplayName Actor) (Utilities|String|ToString(Boolean) (.bsuccessfullysensed Stimulus))) true true "(R=0.000000,G=0.660000,B=1.000000,A=1.000000)" 5.0)
  (AI|Components|Blackboard|SetValueasObject (AI|GetBlackboard 0) (Utilities|Name|MakeLiteralName "Player") Actor))

(event EventBeginPlay
  (|CallParentFunction) ; This node is disabled and will not be called.\nDrag off pins to build functionality.
)

(event Collision|EventActorBeginOverlap
  (params (OtherActor :type Actor%20Object%20Reference)))

(event EventTick
  (params (DeltaSeconds :type Float%20%28single-precision%29)))

(fn ConstructionScript
  (|CallParentFunction))

(fn EVUpdateAIState)