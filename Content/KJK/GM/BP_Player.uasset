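; Player Blueprint on generic team 0 that routes Enhanced Input to interaction, box rewards and skills.
; Interaction input passes the searcher component's target to interaction components on both player and target.
; A BP_Box target also opens a fading-in reward widget with mouse cursor, then gets hidden with collision off.
; Skill inputs toggle the HUD's skill inventory via FlipFlop or fire the first slot through the controller's QuickSlotComponent.
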(event Custom|ResCreateReward
  (params (Targetactor :type Actor%20Object%20Reference))
  (CallFunction|CreateRewardWidget Targetactor))

(event Input|EnhancedActionEvents|EnhancedInputActionIA_Interaction
  (params (ActionValue :type Boolean) (ElapsedSeconds :type Float%20%28double-precision%29) (TriggeredSeconds :type Float%20%28double-precision%29) (InputAction :type Input%20Action%20Object%20Reference :default "/Game/ThirdPerson/Input/Actions/IA_Interaction.IA_Interaction"))
  (:Started
    (bind _targetactor (Default|GetObjectTarget (Variables|Default|GetBP_SearcherComponent)))
    (Default|DoInteract (Variables|Default|GetBP_InteractionComponent) _targetactor)
    (if (Class|GameplayStatics|ObjectIsA _targetactor "/Game/KHC/Item/BP_Box.BP_Box_C")
      (CallFunction|ResCreateReward _targetactor))))

(event EventBeginPlay
  (Utilities|Struct|SetmembersinGenericTeamId (Utilities|Struct|MakeGenericTeamId 0))
  (|CallParentFunction))

(event Collision|EventActorBeginOverlap
  (params (OtherActor :type Actor%20Object%20Reference)))

(event EventTick
  (params (DeltaSeconds :type Float%20%28single-precision%29)))

(event Input|EnhancedActionEvents|EnhancedInputActionIA_Interaction
  (params (ActionValue :type Boolean) (ElapsedSeconds :type Float%20%28double-precision%29) (TriggeredSeconds :type Float%20%28double-precision%29) (InputAction :type Input%20Action%20Object%20Reference :default "/Game/ThirdPerson/Input/Actions/IA_Interaction.IA_Interaction"))
  (:Started
    (bind _targetactor (Default|GetObjectTarget (Variables|Default|GetBP_SearcherComponent)))
    (Utilities|IsValid _targetactor
      (:Is%20Valid
        (Utilities|IsValid (Actor|GetComponentbyClass _targetactor "/Game/SWS/Interaction/BP_InteractionComponent.BP_InteractionComponent_C")
          (:Is%20Valid
            (Default|DoInteract (Actor|GetComponentbyClass _targetactor "/Game/SWS/Interaction/BP_InteractionComponent.BP_InteractionComponent_C") (Components|GetOwner))))))))

(event Input|EnhancedActionEvents|EnhancedInputActionIA_Skill1
  (params (ActionValue :type Vector%202D%20Structure) (ElapsedSeconds :type Float%20%28double-precision%29) (TriggeredSeconds :type Float%20%28double-precision%29) (InputAction :type Input%20Action%20Object%20Reference :default "/Game/ThirdPerson/Input/Actions/IA_Skill1.IA_Skill1"))
  (:Started
    (bind _asbp_player_controller (Utilities|Casting|CastToBP_PlayerController (Components|GetOwner)))
    (Default|UseQuickSlotSkill (Variables|/Game/KJK/GM/BP_PlayerController.BP_PlayerController_C|GetQuickSlotComponent _asbp_player_controller) "NewEnumerator1")))

(event Input|EnhancedActionEvents|EnhancedInputActionIA_Skill_Inventory
  (params (ActionValue :type Vector%202D%20Structure) (ElapsedSeconds :type Float%20%28double-precision%29) (TriggeredSeconds :type Float%20%28double-precision%29) (InputAction :type Input%20Action%20Object%20Reference :default "/Game/ThirdPerson/Input/Actions/IA_Skill_Inventory.IA_Skill_Inventory"))
  (:Started
    (Utilities|FlowControl|FlipFlop
      (:A
        (bind _asquick_slot_hud (Utilities|Casting|CastToQuickSlotHUd (HUD|GetHUD (Game|GetPlayerController 0))))
        (Widget|SetVisibility (Variables|/Game/SWS/QuickSlot/WB_QuickSlot.WB_QuickSlot_C|GetWB_SkillInventory (Variables|/Game/SWS/QuickSlot/QuickSlotHUd.QuickSlotHUd_C|GetQuickSlot _asquick_slot_hud)) "Visible")
        (Default|OpenSkillWindow (Variables|/Game/SWS/QuickSlot/QuickSlotHUd.QuickSlotHUd_C|GetQuickSlot _asquick_slot_hud)))
      (:B
        (Widget|SetVisibility (Variables|/Game/SWS/QuickSlot/WB_QuickSlot.WB_QuickSlot_C|GetWB_SkillInventory (Variables|/Game/SWS/QuickSlot/QuickSlotHUd.QuickSlotHUd_C|GetQuickSlot _asquick_slot_hud)) "Collapsed")
        (Default|CloseSkillWindow (Variables|/Game/SWS/QuickSlot/QuickSlotHUd.QuickSlotHUd_C|GetQuickSlot _asquick_slot_hud))))))

(fn ConstructionScript
  (|CallParentFunction))

(fn CreateRewardWidget
  (params (TargetActor :type Actor%20Object%20Reference))
  (bind _returnvalue (UserInterface|CreateWidget "/Game/KHC/Widget/RewardWidget.RewardWidget_C"))
  (bind _output_get (Variables|Default|SetRewardWidget _returnvalue))
  (UserInterface|Viewport|AddtoViewport _output_get 0)
  (Default|PlayFadein _output_get)
  (Input|SetInputModeGameandUI (Game|GetPlayerController 0) 0 "DoNotLock" true false)
  (Variables|/Script/Engine.PlayerController|SetbShowMouseCursor (Game|GetPlayerController 0) true)
  (CallFunction|HideActor TargetActor))

(fn HideActor
  (params (Target :type Actor%20Object%20Reference))
  (Rendering|SetActorHiddenInGame Target true)
  (Collision|SetActorEnableCollision Target false))