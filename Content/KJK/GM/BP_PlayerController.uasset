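; BP_PlayerController is a player controller that sets up per-player gameplay managers and handles travel to the dungeon.
; On BeginPlay it spawns inventory, store and battle manager actors owned by itself, and adds a skill manager component, storing references to each.
; This setup runs without an authority check, as the SwitchHasAuthority node is unconnected.
; Server_TravelToDungeon issues a servertravel console command to load the Dungeon map.
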(event Custom|Server_TravelToDungeon
  (Development|ExecuteConsoleCommand "servertravel Dungeon" 0))

(event EventBeginPlay
  (bind _returnvalue (Game|SpawnActorfromClass "/Game/KDY/Inventory/BP_InventoryManager.BP_InventoryManager_C" (Transformation|GetActorTransform) "Undefined" "MultiplyWithRoot" 0 0))
  (bind _output_get (Variables|Default|SetInventoryManager _returnvalue))
  (Actor|SetOwner _output_get self)
  (bind _returnvalue_2 (Game|SpawnActorfromClass "/Game/SMH/Blueprints/Tools/BP_StoreManager.BP_StoreManager_C" (Transformation|GetActorTransform) "Undefined" "MultiplyWithRoot" 0 0))
  (bind _output_get_2 (Variables|Default|SetStoreManager _returnvalue_2))
  (Actor|SetOwner _output_get_2 self)
  (bind _returnvalue_3 (Game|SpawnActorfromClass "/Game/KJK/GM/BP_BattleManager.BP_BattleManager_C" (Transformation|GetActorTransform) "Undefined" "MultiplyWithRoot" 0 0))
  (bind _output_get_3 (Variables|Default|SetBattleManager _returnvalue_3))
  (Actor|SetOwner _output_get_3 self)
  (bind _returnvalue_4 (Game|AddComponentbyClass "/Game/SWS/Skill/BP_SkillManagerComponent.BP_SkillManagerComponent_C"))
  (Variables|Default|SetSkillManager _returnvalue_4))

(fn ConstructionScript)