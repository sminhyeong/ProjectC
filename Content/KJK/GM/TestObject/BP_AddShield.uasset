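; BP_AddShield is a test pickup-style actor that grants shield to characters that touch it.
; When its Cube component begins an overlap, the server casts the other actor to BP_BaseCharacter and calls its add-shield event with the SheildAmount variable.
; It then prints the character's name and current shield for debugging; the actor is not destroyed, so each new overlap grants shield again.
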(event OnComponentBeginOverlap(Cube)
  (params (OverlappedComponent :type Primitive%20Component%20Object%20Reference) (OtherActor :type Actor%20Object%20Reference) (OtherComp :type Primitive%20Component%20Object%20Reference) (OtherBodyIndex :type Integer) (bFromSweep :type Boolean) (SweepResult :type Hit%20Result%20Structure%20%28by%20ref%29))
  (Networking|SwitchHasAuthority
    (:Authority
      (bind _asbp_base_character (Utilities|Casting|CastToBP_BaseCharacter OtherActor))
      (Default|EventAddShield _asbp_base_character (Variables|Default|GetSheildAmount))
      (Development|PrintString (Utilities|String|Append "Name" (Utilities|String|ToString(Name) (Variables|/Game/KJK/GM/BP_BaseCharacter.BP_BaseCharacter_C|GetCharacterName _asbp_base_character)) "Shield" (Utilities|String|ToString(Float) (Variables|/Script/ProjectC.CharacterStateComponent|GetCurShield (Variables|/Game/KJK/GM/BP_BaseCharacter.BP_BaseCharacter_C|GetCharacterState _asbp_base_character))))))))

(event EventBeginPlay
  (|CallParentFunction) ; This node is disabled and will not be called.\nDrag off pins to build functionality.
)

(event Collision|EventActorBeginOverlap
  (params (OtherActor :type Actor%20Object%20Reference))
  (|CallParentFunction OtherActor) ; This node is disabled and will not be called.\nDrag off pins to build functionality.
)

(event EventTick
  (params (DeltaSeconds :type Float%20%28single-precision%29))
  (|CallParentFunction DeltaSeconds) ; This node is disabled and will not be called.\nDrag off pins to build functionality.
)

(fn ConstructionScript
  (|CallParentFunction))