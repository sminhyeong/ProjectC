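; BP_MP is a test actor that drains MP from characters who touch it.
; When its Cube component begins overlapping a BaseCharacter, it subtracts UseMPAmount from CurMP in that character's CharacterState, with no clamping.
; It then prints the character's name and remaining MP for debugging.
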(event OnComponentBeginOverlap(Cube)
  (params (OverlappedComponent :type Primitive%20Component%20Object%20Reference) (OtherActor :type Actor%20Object%20Reference) (OtherComp :type Primitive%20Component%20Object%20Reference) (OtherBodyIndex :type Integer) (bFromSweep :type Boolean) (SweepResult :type Hit%20Result%20Structure%20%28by%20ref%29))
  (bind _asbase_character (Utilities|Casting|CastToBaseCharacter OtherActor))
  (bind _output_get (Variables|/Script/ProjectC.CharacterStateComponent|SetCurMP (Variables|/Game/KJK/GM/BaseCharacter.BaseCharacter_C|GetCharacterState _asbase_character) (- (Variables|/Script/ProjectC.CharacterStateComponent|GetCurMP (Variables|/Game/KJK/GM/BaseCharacter.BaseCharacter_C|GetCharacterState _asbase_character)) (Variables|Default|GetUseMP%20Amount))))
  (Development|PrintString (Utilities|String|Append "Name" (Utilities|String|ToString(Name) (Variables|/Game/KJK/GM/BaseCharacter.BaseCharacter_C|GetCharacterName _asbase_character)) "CurMP" (Utilities|String|ToString(Float) _output_get))))

(event EventBeginPlay
  (|CallParentFunction) ; This node is disabled and will not be called.\nDrag off pins to build functionality.
)

(event Collision|EventActorBeginOverlap
  (params (OtherActor :type Actor%20Object%20Reference))
  (|CallParentFunction OtherActor) ; This node is disabled and will not be called.\nDrag off pins to build functionality.
)

(event EventTick
  (params (DeltaSeconds :type Float%20%28single-precision%29))
  (|CallParentFunction DeltaSeconds) ; This node is disabled and will not be called.\nDrag off pins to build functionality.
)

(fn ConstructionScript
  (|CallParentFunction))