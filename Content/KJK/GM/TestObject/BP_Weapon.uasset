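; BP_Weapon is a test weapon that deals melee-style area damage for its owning Character.
; Notify picks a point in front of the Character and passes it through ReqNotify to EventNotify, which sphere-overlaps object types chosen by the Player or Monster tag.
; Each overlapped actor takes fixed damage, then the empty ResNotify hook fires.
; A debug sphere marks hits; team filtering is a placeholder, and a note plans a socket line trace.
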(event Custom|ReqNotify
  (params (SpherePos :type Vector))
  (CallFunction|EventNotify SpherePos))

(event Custom|ResNotify)

(fn ConstructionScript)

(fn EventNotify
  (params (SpherePos :type Vector))
  (if (Actor|ActorHasTag (Variables|Default|GetCharacter) "Player")
    (Utilities|Array|Add (LocalVariables|GetNewLocalVar_0) "ObjectTypeQuery9")
    ;[0.15 0.15 0.15 0.5] 소켓라인트레이스로 바꾸기
    (bind (_outactors _returnvalue) (Collision|SphereOverlapActors SpherePos 1e+02 (LocalVariables|GetNewLocalVar_0) 0 (Utilities|Array|MakeArray (Variables|Default|GetAs%20BP%20Player)) :!label _label))
    (if _returnvalue
      (Rendering|Debug|DrawDebugSphere SpherePos 1e+02 12 "(R=1.000000,G=0.000000,B=0.000000,A=1.000000)" 3.0)
      ;[0.15 0.15 0.15 0.5] 상대
      (for _array_element _outactors
        ;[0.15 0.15 0.15 0.5] 팀 처리
        (if true
          (Game|Damage|ApplyDamage _array_element 5.0 (Game|GetInstigatorController (Variables|Default|GetCharacter)) self)
          (CallFunction|ResNotify))))
    (elif (Actor|ActorHasTag (Variables|Default|GetCharacter) "Monster")
      (Utilities|Array|Add (LocalVariables|GetNewLocalVar_0) "ObjectTypeQuery8")
      (goto _label))))

(fn Notify
  (bind _character (Variables|Default|GetCharacter)
    (:then
      (CallFunction|ReqNotify (+ (Transformation|GetActorLocation _character) (* (Transformation|GetActorForwardVector _character) 1.5e+02))))
    (:else)))