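; BP_NetworkManager is an Actor blueprint that stores the client's user data and login state.
; Simple setter and getter functions write and read the ClientUserData and IsLogin variables, with each setter returning the stored value.
; Despite the name, its graphs contain no networking logic, and the event graph and construction script are empty.
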(event EventBeginPlay)

(event Collision|EventActorBeginOverlap
  (params (OtherActor :type Actor%20Object%20Reference)))

(event EventTick
  (params (DeltaSeconds :type Float%20%28single-precision%29)))

(fn ConstructionScript)

(fn SetUserData
  (params (ClientUserData :type Account%20Login%20Response%20Structure))
  (bind _output_get (Variables|Default|SetClientUserData ClientUserData))
  (return _output_get))

(fn GetUserData
  (return (Variables|Default|GetClientUserData)))

(fn SetIsLogin
  (params (IsLogin :type Boolean))
  (bind _output_get (Variables|Default|SetIsLogin IsLogin))
  (return _output_get))

(fn IsClientLogin
  (return (Variables|Default|GetIsLogin)))