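; Test game state for an SMH entry level that exercises the client's connection to the game server.
; On BeginPlay it shows a NetConnectTestWidget, binds to the game instance NetworkManager's connection state event, and connects to a hardcoded host and port.
; The bound handler recolors the widget for each connection state, with Connecting and Reconnecting sharing one color.
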(event EventBeginPlay
  (bind _asbp_game_instance (Utilities|Casting|CastToBP_GameInstance (Game|GetGameInstance)))
  (bind _returnvalue (UserInterface|CreateWidget "/Game/SMH/Blueprints/Tools/NetConnectTestWidget.NetConnectTestWidget_C"))
  (bind _output_get (Variables|Default|SetConnectWidget _returnvalue))
  (UserInterface|Viewport|AddtoViewport _output_get 0)
  (EventDispatchers|BindEventtoOnConnectionStateChanged (Default|GetNetworkManager _asbp_game_instance) (EventDispatchers|CreateEvent :!event BPSMHTESTEntryGameStateAutoGenFunc))
  (Class|NetworkManager|ConnecttoServer (Default|GetNetworkManager _asbp_game_instance) "smhportopolioserver.tplinkdns.com" 36930))

(fn ConstructionScript)

(fn BPSMHTESTEntryGameStateAutoGenFunc
  (params (NewState :type ENetConnectionState%20Enum :default "Disconnected"))
  (switch Utilities|FlowControl|Switch|SwitchonENetConnectionState NewState
    (:Disconnected
      (Default|ChangeConnectState (Variables|Default|GetConnectWidget) "(R=1.000000,G=0.000000,B=0.000000,A=1.000000)"))
    (:Connecting
      (Default|ChangeConnectState (Variables|Default|GetConnectWidget) "(R=0.000000,G=1.000000,B=0.000000,A=1.000000)" :!label _label))
    (:Connected
      (Default|ChangeConnectState (Variables|Default|GetConnectWidget) "(R=0.000000,G=0.000000,B=1.000000,A=1.000000)"))
    (:Reconnecting
      (goto _label))
    (:Failed
      (Default|ChangeConnectState (Variables|Default|GetConnectWidget) "(R=0.000000,G=0.000000,B=0.000000,A=1.000000)"))))