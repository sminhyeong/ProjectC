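; Test GameMode that exposes store and player inventory operations: listing shop items, reading inventory or item info, and adding, removing or setting item quantities.
; Each function casts the GameInstance to BP_GameInstance and forwards to its Network Manager, returning the result and message.
; A failed cast or validity check returns false with an error message.
; GetStoreItemList's validity check has no input shown, unlike the others; the event graph is empty.
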(event EventBeginPlay)

(event EventTick
  (params (DeltaSeconds :type Float%20%28single-precision%29)))

(fn ConstructionScript)

(fn GetStoreItemList
  (params (ShopID :type Integer))
  (bind _asbp_game_instance (Utilities|Casting|CastToBP_GameInstance (Game|GetGameInstance))
    (:then
      (Utilities|IsValid 0
        (:Is%20Valid
          (bind (_outshopitems _outmessage _returnvalue) (Class|NetworkManager|GetStoreItemList (Default|GetNetworkManager _asbp_game_instance) ShopID))
          (return _outshopitems _outmessage _returnvalue))
        (:Is%20Not%20Valid
          _)))
    (:CastFailed
      _))
  (return 0 "Is Not Valid Network Manager" false))

(fn GetPlayerInventory
  (params (UserID :type Integer))
  (bind _asbp_game_instance (Utilities|Casting|CastToBP_GameInstance (Game|GetGameInstance))
    (:then
      (Utilities|IsValid (Default|GetNetworkManager _asbp_game_instance)
        (:Is%20Valid
          (bind (_outinventoryitems _outmessage _returnvalue) (Class|NetworkManager|GetPlayerInventory (Default|GetNetworkManager _asbp_game_instance) UserID))
          (return _outinventoryitems _outmessage _returnvalue))
        (:Is%20Not%20Valid
          _)))
    (:CastFailed
      _))
  (return 0 "Is Not Valid Network Manager" false))

(fn GetSingleItemInfo
  (params (UserID :type Integer) (ItemID :type Integer))
  (bind _asbp_game_instance (Utilities|Casting|CastToBP_GameInstance (Game|GetGameInstance))
    (:then
      (Utilities|IsValid (Default|GetNetworkManager _asbp_game_instance)
        (:Is%20Valid
          (bind (_outiteminfo _outmessage _returnvalue) (Class|NetworkManager|GetSingleItemInfo (Default|GetNetworkManager _asbp_game_instance) UserID ItemID))
          (return _outiteminfo _outmessage _returnvalue))
        (:Is%20Not%20Valid
          _)))
    (:CastFailed
      _))
  (return "" "Is Not Valid Network Manager" false))

(fn AddItemtoInventory
  (params (UserID :type Integer) (ItemID :type Integer) (ItemCount :type Integer))
  (bind _asbp_game_instance (Utilities|Casting|CastToBP_GameInstance (Game|GetGameInstance))
    (:then
      (Utilities|IsValid (Default|GetNetworkManager _asbp_game_instance)
        (:Is%20Valid
          (bind (_outmessage _returnvalue) (Class|NetworkManager|AddItemtoInventory (Default|GetNetworkManager _asbp_game_instance) UserID ItemID ItemCount))
          (return _outmessage _returnvalue))
        (:Is%20Not%20Valid
          _)))
    (:CastFailed
      _))
  (return "Is Not Valid Network Manager " false))

(fn RemoveItemfromInventory
  (params (UserID :type Integer) (ItemID :type Integer) (ItemCount :type Integer))
  (bind _asbp_game_instance (Utilities|Casting|CastToBP_GameInstance (Game|GetGameInstance))
    (:then
      (Utilities|IsValid (Default|GetNetworkManager _asbp_game_instance)
        (:Is%20Valid
          (bind (_outmessage _returnvalue) (Class|NetworkManager|RemoveItemfromInventory (Default|GetNetworkManager _asbp_game_instance) UserID ItemID ItemCount))
          (return _outmessage _returnvalue))
        (:Is%20Not%20Valid
          _)))
    (:CastFailed
      _))
  (return "Is Not valid Network Manager" false))

(fn SetItemQuantity
  (params (UserID :type Integer) (ItemID :type Integer) (NewQuantity :type Integer))
  (bind _asbp_game_instance (Utilities|Casting|CastToBP_GameInstance (Game|GetGameInstance))
    (:then
      (Utilities|IsValid (Default|GetNetworkManager _asbp_game_instance)
        (:Is%20Valid
          (bind (_outmessage _returnvalue) (Class|NetworkManager|SetItemQuantity (Default|GetNetworkManager _asbp_game_instance) UserID ItemID NewQuantity))
          (return _outmessage _returnvalue))
        (:Is%20Not%20Valid
          _)))
    (:CastFailed
      _))
  (return "Is Not valid Network Manager" false))