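; Player controller store manager that opens a shop UI and handles item purchases and sales.
; The local player's instance creates WBP_Store, binds to it, and switches to UI-only input when the shop opens.
; Request events query or transact through BP_LobbyGM on the authority game mode, and response events open the store or dispatch gold updates.
; Inventory refreshes go through the controller's InventoryManager into the store's inventory window.
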(event Custom|StoreItemListRequest
  (params (ShopID :type Integer))
  (bind _asbp_lobby_gm (Utilities|Casting|CastToBP_LobbyGM (Variables|/Script/Engine.GameStateBase|GetAuthorityGameMode (Game|GetGameState)))
    (:then
      (bind (_outshopitems _outmessage _returnvalue) (Default|GetStoreItemList _asbp_lobby_gm ShopID))
      (CallFunction|OpenStoreEvent _outshopitems _outmessage _returnvalue))
    (:CastFailed
      (CallFunction|OpenStoreEvent 0 "Don't Request Store ItemList" false))))

(event Custom|OpenStoreEvent
  (params (ItemList :type Array%20of%20Account%20Item%20Info%20Structures) (Out%20Message :type String) (IsSuccess :type Boolean))
  (bind _returnvalue (Game|GetPlayerController 0))
  (if IsSuccess
    (bind _bissuccess (Default|OpenStoreWidget (Variables|Default|GetStoreWidget) ItemList))
    (if _bissuccess
      (Input|SetInputModeUIOnly _returnvalue 0 "DoNotLock" true)
      (Variables|/Script/Engine.PlayerController|SetbShowMouseCursor _returnvalue true))
    (else
      (Development|PrintString Out%20Message))))

(event EventBeginPlay
  (if (== (Components|GetOwner) (Game|GetPlayerController 0))
    (bind _returnvalue (UserInterface|CreateWidget "/Game/KDY/WBP_Store.WBP_Store_C"))
    (bind _output_get (Variables|Default|SetStoreWidget _returnvalue))
    (UserInterface|Viewport|AddtoViewport _output_get 0)
    (Widget|SetVisibility (Variables|Default|GetStoreWidget) "Collapsed")
    (Class|BPIInvenorStoreWidget|BindwithManager(Message) (Variables|Default|GetStoreWidget) self)
    (EventDispatchers|BindEventtoDPUpdateInventoryItem (Variables|Default|GetStoreWidget) (EventDispatchers|CreateEvent :!event Custom|CustomEvent))))

(event Custom|SellRequest
  (params (UserID :type Integer) (ItemID :type Integer) (ItemCount :type Integer) (StoreID :type Integer))
  (bind _asbp_lobby_gm (Utilities|Casting|CastToBP_LobbyGM (Variables|/Script/Engine.GameStateBase|GetAuthorityGameMode (Game|GetGameState)))
    (:then
      (bind (_outnewgold _outmessage _returnvalue) (Default|SellItem _asbp_lobby_gm UserID StoreID ItemID ItemCount))
      (CallFunction|SellRespon _outnewgold _outmessage _returnvalue))
    (:CastFailed
      (CallFunction|SellRespon 0 "Don't Request SellItem" false))))

(event Custom|SellRespon
  (params (Out%20New%20Gold :type Integer) (Out%20Message :type String) (IsSuccess :type Boolean))
  (Default|CallDPUpdateGold Out%20New%20Gold Out%20Message IsSuccess))

(event Custom|PurchseRequest
  (params (UserID :type Integer) (ItemID :type Integer) (ItemCount :type Integer) (StoreID :type Integer))
  (bind _asbp_lobby_gm (Utilities|Casting|CastToBP_LobbyGM (Variables|/Script/Engine.GameStateBase|GetAuthorityGameMode (Game|GetGameState)))
    (:then
      (bind (_outnewgold _outmessage _returnvalue) (Default|PurchaseItem _asbp_lobby_gm UserID StoreID ItemID ItemCount))
      (CallFunction|PurchaseRespon _outnewgold _outmessage _returnvalue))
    (:CastFailed
      (CallFunction|PurchaseRespon 0 "Don't Request PurchaseItem" false))))

(event Custom|PurchaseRespon
  (params (OutNewGold :type Integer) (OutMessage :type String) (IsSueccess :type Boolean))
  (Default|CallDPUpdateGold OutNewGold OutMessage IsSueccess))

(event Custom|UpdateInventoryReq
  (params (User_Id :type Integer))
  (bind _asbp_player_controller (Utilities|Casting|CastToBP_PlayerController (Components|GetOwner)))
  (Class|InventoryManager|UpdateInventoryData (Variables|/Game/KJK/GM/BP_PlayerController.BP_PlayerController_C|GetInventoryManager _asbp_player_controller) User_Id)
  (CallFunction|UpdateInventoryRes))

(event Custom|UpdateInventoryRes
  (bind _asbp_player_controller (Utilities|Casting|CastToBP_PlayerController (Components|GetOwner)))
  (Class|InventoryManager|S2CUpdateInventoryWidget (Variables|/Game/KJK/GM/BP_PlayerController.BP_PlayerController_C|GetInventoryManager _asbp_player_controller) (Variables|/Game/KDY/WBP_Store.WBP_Store_C|GetWBP_InventoryWindow (Variables|Default|GetStoreWidget))))

(event Custom|CustomEvent
  (params (UserId :type Integer))
  (CallFunction|UpdateInventoryReq UserId))

(fn ConstructionScript)

(fn OpenStore
  (params (ShopID :type Integer))
  (Default|SetMoneyatWidget (Variables|Default|GetStoreWidget))
  (bind _output_get (Variables|Default|SetStoreId ShopID))
  (CallFunction|StoreItemListRequest _output_get))

(fn SellItem
  (params (UserID :type Integer) (ItemID :type Integer) (ItemCount :type Integer) (StoreID :type Integer))
  (CallFunction|SellRequest UserID ItemID ItemCount StoreID))

(fn PurchaseItem
  (params (UserID :type Integer) (ItemID :type Integer) (ItemCount :type Integer) (StoreID :type Integer))
  (CallFunction|PurchseRequest UserID ItemID ItemCount StoreID))

(fn GetInventoryDatafromInventoryManager
  (bind _asbp_player_controller (Utilities|Casting|CastToBP_PlayerController (Components|GetOwner)))
  (bind _asbp_game_instance (Utilities|Casting|CastToBP_GameInstance (Game|GetGameInstance)))
  (Default|UpdateInventoryReq (Variables|/Game/KJK/GM/BP_PlayerController.BP_PlayerController_C|GetInventoryManager _asbp_player_controller) (Class|NetworkManager|GetCurrentUserID (Class|NetGameInstanceBase|GetNetworkManager _asbp_game_instance)))
  (return (Variables|/Script/ProjectC.InventoryManager|GetWeaponList (Variables|/Game/KJK/GM/BP_PlayerController.BP_PlayerController_C|GetInventoryManager _asbp_player_controller)) (Variables|/Script/ProjectC.InventoryManager|GetArmorList (Variables|/Game/KJK/GM/BP_PlayerController.BP_PlayerController_C|GetInventoryManager _asbp_player_controller)) (Variables|/Script/ProjectC.InventoryManager|GetConsumeList (Variables|/Game/KJK/GM/BP_PlayerController.BP_PlayerController_C|GetInventoryManager _asbp_player_controller))))