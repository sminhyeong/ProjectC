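; BP_InteractionComponent is an actor component that passes interaction requests from its owner to a target actor's own interaction component.
; DoInteract validates the target and sends a request, which HasInteraction forwards as a response if the target's component implements BPI_Interactable.
; The response is test code that overwrites every mesh material on interactor and target Characters, using a different material for each.
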(event Custom|Req_Interact
  (params (Interactor :type Actor%20Object%20Reference) (TargetActor :type Actor%20Object%20Reference))
  (CallFunction|HasInteraction Interactor TargetActor))

(event Custom|Res_Interact
  (params (Interactor :type Actor%20Object%20Reference) (TargetActor :type Actor%20Object%20Reference))
  ;[0.15 0.15 0.15 0.5] 테스트용
  (bind _ascharacter (Utilities|Casting|CastToCharacter Interactor))
  (for (_ _array_index) (Rendering|Material|GetMaterials (Variables|/Script/Engine.Character|GetMesh _ascharacter))
    (Rendering|Material|SetMaterial (Variables|/Script/Engine.Character|GetMesh _ascharacter) _array_index "/Engine/EngineMeshes/BackgroundMaterial.BackgroundMaterial"))
  (bind _ascharacter_2 (Utilities|Casting|CastToCharacter TargetActor))
  (for (_ _array_index_2) (Rendering|Material|GetMaterials (Variables|/Script/Engine.Character|GetMesh _ascharacter_2))
    (Rendering|Material|SetMaterial (Variables|/Script/Engine.Character|GetMesh _ascharacter_2) _array_index_2 "/Engine/MapTemplates/Materials/BasicAsset01.BasicAsset01")))

(fn DoInteract
  (params (TargetActor :type Actor%20Object%20Reference))
  (Utilities|IsValid TargetActor
    (:Is%20Valid
      (CallFunction|ReqInteract (Components|GetOwner) TargetActor)
      (return false))))

(fn HasInteraction
  (params (Interactor :type Actor%20Object%20Reference) (TargetActor :type Actor%20Object%20Reference))
  (bind _returnvalue (Actor|GetComponentbyClass TargetActor "BP_InteractionComponent_C"))
  (if (Utilities|DoesObjectImplementInterface _returnvalue "/Game/SWS/Interaction/BPI_Interactable.BPI_Interactable_C")
    (CallFunction|ResInteract _returnvalue Interactor TargetActor)
    (return false)))