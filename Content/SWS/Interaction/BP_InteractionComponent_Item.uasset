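; BP_InteractionComponent_Item is an item interaction component that currently holds placeholder test behavior.
; On ResInteract it swaps every material on the owner's static mesh component to AnimSharingBlue and prints the interactor and target names to screen.
; HasInteraction always returns false.
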(event EventResInteract
  (params (Interactor :type Actor%20Object%20Reference) (TargetActor :type Actor%20Object%20Reference))
  (bind _returnvalue (Components|GetOwner))
  (bind _returnvalue_2 (Actor|GetComponentbyClass _returnvalue "/Script/Engine.StaticMeshComponent"))
  ;[0.15 0.15 0.15 0.5] 테스트용- 머터리얼 교체
  (for (_ _array_index) (Rendering|Material|GetMaterials _returnvalue_2)
    (Rendering|Material|SetMaterial _returnvalue_2 _array_index "/AnimationSharing/AnimSharingBlue.AnimSharingBlue"))
  (Development|PrintString (Utilities|String|Append "  Interactor: " (Utilities|GetDisplayName Interactor) "  TargetItem: " (Utilities|GetDisplayName TargetActor)) true true "(R=0.816845,G=0.393235,B=1.000000,A=1.000000)" 6e+01))

(fn HasInteraction
  (params (Interactor :type Actor%20Object%20Reference) (TargetActor :type Actor%20Object%20Reference))
  (return false))