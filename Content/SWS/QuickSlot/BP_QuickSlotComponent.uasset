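; Quick slot component that holds the player's equipped skills and uses them by slot index through the player character's BP_SkillManagerComponent.
; On BeginPlay it binds to the manager's skill-use event, creates a slot from DT_Skill's "Empty" row and fills it from the skill list.
; Set and swap broadcast UpdateQuickSlot, while removal edits the HUD tile view directly.
; It also binds to each skill icon's drag-and-drop event.
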(event EventBeginPlay
  (CallFunction|BindSkillManager)
  (CallFunction|CreateSkillSlots 1)
  (CallFunction|InitDefaultQuickSlot 1)
  (CallFunction|BindQuickSlotSkillUI))

(fn SetQuickSlotSkill
  (params (SlotIndex :type Integer) (ST_SkillData :type ST%20Skill%20Data%20Structure%20%28by%20ref%29))
  (bind _skillmanager (Variables|Default|GetSkillManager))
  (bind _array_index (Default|FindinSkillList _skillmanager ST_SkillData))
  (bind _skilllist (Default|GetSkillList _skillmanager))
  (bind _output (Utilities|Array|Get(acopy) _skilllist _array_index))
  (if (Utilities|Array|ContainsItem _skilllist _output)
    (Utilities|Array|SetArrayElem (Variables|Default|GetSkills_QuickSlot) SlotIndex _output true)
    (Default|CallEventDispatcherUpdateQuickSlot)))

(fn RemoveQuickSlotSkill
  (params (Index :type Integer) (SkillData :type ST%20Skill%20Data%20Structure))
  (bind _quick_slot (Variables|Default|GetQuick%20Slot))
  (bind _tile_skill_quickslot (Variables|/Game/SWS/QuickSlot/WB_QuickSlot.WB_QuickSlot_C|GetTile_Skill_QuickSlot _quick_slot))
  (bind _returnvalue (Class|ListView|GetItemat _tile_skill_quickslot Index))
  (Utilities|Array|SetArrayElem :TargetArray (Variables|Default|GetSkills_QuickSlot) :Index Index)
  (Development|PrintString (Utilities|GetDisplayName _returnvalue))
  (Class|ListView|RemoveItem _tile_skill_quickslot _returnvalue))

(fn GetSkillData
  (params (Index :type Integer))
  (bind _skills_quickslot (Variables|Default|GetSkills_QuickSlot))
  (if (> (Utilities|Array|Length _skills_quickslot) Index)
    (return (Utilities|Array|Get(acopy) _skills_quickslot Index))))

(fn UpdateSlotSkill
  (params (CurrentSkill :type ST%20Current%20Skill%20Data%20Structure))
  (bind _array_index (CallFunction|FindinSlot (.SkillData (Utilities|Struct|BreakST_CurrentSkillData CurrentSkill))))
  (Utilities|Array|SetArrayElem (Variables|Default|GetSkills_QuickSlot) _array_index CurrentSkill))

(fn FindinSlot
  (params (ST_SkillData :type ST%20Skill%20Data%20Structure%20%28by%20ref%29))
  (for (_array_element _array_index) (CallFunction|GetSkillList)
    (if (== (.SKilll_ID (Utilities|Struct|BreakST_SkillData (.SkillData (Utilities|Struct|BreakST_CurrentSkillData _array_element)))) (.SKilll_ID (Utilities|Struct|BreakST_SkillData ST_SkillData)))
      (return _array_index)))
  (return -1))

(fn GetSkillList
  (return (Variables|Default|GetSkills_QuickSlot)))

(fn BindSkillManager
  (bind _ascharacter (Utilities|Casting|CastToCharacter (Game|Player|GetPlayerPawn 0)))
  (bind _output_get (Variables|Default|SetSkillManager (Actor|GetComponentbyClass _ascharacter "/Game/SWS/Skill/BP_SkillManagerComponent.BP_SkillManagerComponent_C")))
  (EventDispatchers|BindEventtoEventDispatcherUseSkill _output_get (EventDispatchers|CreateEvent :!event UpdateSlotSkill)))

(fn InitDefaultQuickSlot
  (params (Count :type Integer))
  (bind _asquick_slot_hud (Utilities|Casting|CastToQuickSlotHUd (HUD|GetHUD (Game|GetPlayerController 0))))
  (Variables|Default|SetQuick%20Slot (Variables|/Game/SWS/QuickSlot/QuickSlotHUd.QuickSlotHUd_C|GetQuickSlot _asquick_slot_hud))
  (for (_array_element _array_index) (Default|GetSkillList (Variables|Default|GetSkillManager))
    (if (< _array_index (Math|Integer|Clamp(Integer) Count 0 4))
      (CallFunction|SetQuickSlotSkill _array_index (.SkillData (Utilities|Struct|BreakST_CurrentSkillData _array_element))))))

(fn UseQuickSlotSkill
  (params (SlotType :type EN_SlotType%20Enum :default "NewEnumerator0") (Index :type Integer))
  (bind _output (CallFunction|GetSkillData Index))
  (bind _skilldata (Utilities|Struct|BreakST_CurrentSkillData _output))
  (if (Utilities|IsValidClass (.SKill_Class (Utilities|Struct|BreakST_SkillData _skilldata)))
    (Default|TryUseSkill (Variables|Default|GetSkillManager) _skilldata)))

(fn SwapQuickSlot
  (params (From :type Integer) (To :type Integer))
  (Utilities|Array|Swap (Variables|Default|GetSkills_QuickSlot) From To)
  (Default|CallEventDispatcherUpdateQuickSlot))

(fn CreateSkillSlots
  (params (Count :type Integer))
  (for _index (range 0 (- Count 1))
    (bind _returnvalue (Utilities|GetDataTableRow "/Game/SWS/Skill/DT_Skill.DT_Skill" "Empty")
      (:then
        (Utilities|Array|Add (Variables|Default|GetSkills_QuickSlot) (Utilities|Struct|MakeST_CurrentSkillData _returnvalue 0.0))))))

(fn BindQuickSlotSkillUI
  (for _array_element (Class|ListView|GetListItems (Variables|/Game/SWS/QuickSlot/WB_QuickSlot.WB_QuickSlot_C|GetTile_Skill_QuickSlot (Variables|Default|GetQuick%20Slot)))
    (bind _aswb_icon_skill (Utilities|Casting|CastToWB_Icon_Skill _array_element))
    (EventDispatchers|BindEventtoEventDispatcherDragandDrop _aswb_icon_skill (EventDispatchers|CreateEvent :!event SwapQuickSlot))))