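; Searcher component that detects actors around its owner and keeps the closest one as TargetActor.
; On BeginPlay it adds a sphere collision of configurable radius on a custom trace channel to the owner.
; Bound overlap events maintain ActorList, seeded with initial overlaps minus the owner.
; A looping timer picks the nearest actor within the radius, and GetObjectTargets prints and returns the whole list.
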(event OnComponentBeginOverlap(Collision)
  (params (OverlappedComponent :type Primitive%20Component%20Object%20Reference) (OtherActor :type Actor%20Object%20Reference) (OtherComp :type Primitive%20Component%20Object%20Reference) (OtherBodyIndex :type Integer) (bFromSweep :type Boolean) (SweepResult :type Hit%20Result%20Structure%20%28by%20ref%29))
  ;[0.15 0.15 0.15 0.5] 해당 이벤트 작동X. 커스텀 이벤트 따로 바인드해서 사용중
  (Utilities|IsValid OtherActor
    (:Is%20Valid
      (Development|PrintString "Hello"))))

(event Custom|On%20Component%20Begin%20Overlap%28Collision%29
  (params (OverlappedComponent :type Primitive%20Component%20Object%20Reference) (OtherActor :type Actor%20Object%20Reference) (OtherComp :type Primitive%20Component%20Object%20Reference) (OtherBodyIndex :type Integer) (bFromSweep :type Boolean) (SweepResult :type Hit%20Result%20Structure%20%28by%20ref%29))
  (Utilities|Array|AddUnique (Variables|Default|GetActorList) OtherActor))

(event Custom|On%20Component%20End%20Overlap%28Collision%29
  (params (OverlappedComponent :type Primitive%20Component%20Object%20Reference) (OtherActor :type Actor%20Object%20Reference) (OtherComp :type Primitive%20Component%20Object%20Reference) (OtherBodyIndex :type Integer))
  (Utilities|Array|RemoveItem (Variables|Default|GetActorList) OtherActor))

(event EventBeginPlay
  (bind _returnvalue (Game|AddComponentbyClass (Components|GetOwner) "/Script/Engine.SphereComponent" false))
  (bind _output_get (Variables|Default|SetCollision _returnvalue))
  (Collision|SetCollisionObjectType _output_get "ECC_GameTraceChannel1")
  (Components|Sphere|SetSphereRadius (Variables|Default|GetCollision) (Variables|Default|GetRadius) true)
  (CallFunction|BindEvnentOverlap)
  (Utilities|Time|SetTimerbyFunctionName 0 "RepeatSearchingTarget" 0.1 true))

(fn GetObjectTarget
  (if (Utilities|Array|IsNotEmpty (Variables|Default|GetActorList))
    (LocalVariables|SetClosestDistance (Variables|Default|GetRadius))
    (LocalVariables|SetClosest 0)
    (for _array_element (Variables|Default|GetActorList)
      (if (< (Transformation|GetDistanceTo _array_element (Components|GetOwner)) (LocalVariables|GetClosestDistance))
        (LocalVariables|SetClosestDistance (Transformation|GetDistanceTo _array_element (Components|GetOwner)))
        (LocalVariables|SetClosest _array_element)))
    (return (LocalVariables|GetClosest))
    (else
      (return 0))))

(fn GetObjectTargets
  (bind _actorlist (Variables|Default|GetActorList))
  (for _array_element _actorlist
    (Development|PrintString (Utilities|GetDisplayName _array_element)))
  (return _actorlist))

(fn BindEvnentOverlap
  (bind _collision (Variables|Default|GetCollision))
  (Collision|BindEventtoOnComponentBeginOverlap _collision (EventDispatchers|CreateEvent :!event Custom|On%20Component%20Begin%20Overlap%28Collision%29))
  (Collision|BindEventtoOnComponentEndOverlap _collision (EventDispatchers|CreateEvent :!event Custom|On%20Component%20End%20Overlap%28Collision%29))
  ;[0.15 0.15 0.15 0.5] 겹친상태로 시작시. 소유 액터를 제외
  (bind _output_get (Variables|Default|SetActorList (Collision|GetOverlappingActors _collision 0 :!class /Script/Engine.PrimitiveComponent)))
  (Utilities|Array|RemoveItem _output_get (Components|GetOwner)))

(fn RepeatSearchingTarget
  (bind _targetactor (CallFunction|GetObjectTarget))
  (bind _output_get (Variables|Default|SetTargetActor _targetactor))
  (Utilities|IsValid _output_get))