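; BP_RotationBall is a short-lived skill actor: a ball that orbits its instigator and damages what it passes.
; Each tick it snaps to the instigator's location and yaws a SpringArm at constant speed to swing the ball around.
; An accumulated-time throttle in DoDamage periodically applies radial damage at the mesh's position, ignoring the instigator.
; A lifespan set on BeginPlay removes it, and DoEnd is empty.
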(event EventBeginPlay
  (|CallParentFunction)
  (Actor|SetLifeSpan 4.0))

(event EventTick
  (params (DeltaSeconds :type Float%20%28single-precision%29))
  (Utilities|FlowControl|Sequence
    (:then_0
      (Transformation|AddRelativeRotation (Variables|Default|GetSpringArm) (Math|Rotator|MakeRotator 0.0 0.0 (* DeltaSeconds 1.8e+02)) false false))
    (:then_1
      (Transformation|SetActorLocation (Transformation|GetActorLocation (Game|GetInstigator)) false false))
    (:then_2
      (CallFunction|DoDamage DeltaSeconds))))

(fn ConstructionScript)

(fn DoEnd)

(fn DoDamage
  (params (DeltaSeconds :type Float%20%28double-precision%29))
  (bind _output_get (Variables|Default|SetDamageDelay (+ DeltaSeconds (Variables|Default|GetDamageDelay))))
  (if (> _output_get 0.1)
    (Variables|Default|SetDamageDelay 0.0)
    (Game|Damage|ApplyRadialDamage 1e+01 (Transformation|GetWorldLocation (Variables|Default|GetStaticMesh_0)) 1e+02 0 (Utilities|Array|MakeArray (Game|GetInstigator)) self (Pawn|GetController (Game|GetInstigator)) false "ECC_Visibility")))