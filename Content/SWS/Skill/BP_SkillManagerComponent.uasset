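; Character skill manager component that tracks cooldowns and casts skills defined in DT_Skill.
; On BeginPlay, the authority fills the skill list from every table row and binds the ready dispatcher.
; Tick counts each unready skill's elapsed time up toward its cooldown, firing update and ready dispatchers.
; ReqUseSkill resets a ready skill's timer and spawns its actor at the owner's transform, identically for all handled skill types; cost is stored but never deducted.
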(event Custom|ReqUseSkill
  (params (ST_SkillData :type ST%20Skill%20Data%20Structure%20%28by%20ref%29))
  (CallFunction|TryUseSkill ST_SkillData))

(event EventBeginPlay
  (Networking|SwitchHasAuthority
    (:Authority
      (bind _ascharacter (Utilities|Casting|CastToCharacter (Components|GetOwner)))
      (Variables|Default|SetOwner _ascharacter)
      (bind _outrownames (DataTable|GetDataTableRowNames "/Game/SWS/Skill/DT_Skill.DT_Skill"))
      (for _array_element _outrownames
        (bind _returnvalue (Utilities|GetDataTableRow "/Game/SWS/Skill/DT_Skill.DT_Skill" _array_element)
          (:then
            (CallFunction|AddSkill _returnvalue))))
      (EventDispatchers|BindEventtoEventDispatcherReadytoSkill (EventDispatchers|CreateEvent :!event UpdateReady)))))

(event EventTick
  (params (DeltaSeconds :type Float%20%28single-precision%29))
  (for _array_element (Variables|Default|GetSkillList_Entire)
    (if (not (CallFunction|IsReady (Utilities|Array|Get(acopy) (Variables|Default|GetSkillList_Entire) (CallFunction|FindinSkillList (.SkillData (Utilities|Struct|BreakST_CurrentSkillData _array_element))))))
      (CallFunction|UpdateSkillCooltime (Utilities|Array|Get(acopy) (Variables|Default|GetSkillList_Entire) (CallFunction|FindinSkillList (.SkillData (Utilities|Struct|BreakST_CurrentSkillData _array_element)))))
      (Default|CallEventDispatcherUpdateSkill))))

(fn TryUseSkill
  (params (SkillData :type ST%20Skill%20Data%20Structure))
  (bind _array_index (CallFunction|FindinSkillList SkillData))
  (bind _owner (Variables|Default|GetOwner))
  (bind _skilllist_entire (Variables|Default|GetSkillList_Entire))
  (bind _output (Utilities|Array|Get(acopy) _skilllist_entire _array_index))
  (if (Utilities|IsValidClass (.SKill_Class (Utilities|Struct|BreakST_SkillData SkillData)))
    ;[0.15 0.15 0.15 0.5] 조건 확인
    (if (CallFunction|IsReady _output)
      ;[0.15 0.15 0.15 0.5] 스킬 시전시 처리 부분 (ex 쿨타임, 마나소모)
      (bind _structout (Utilities|Struct|SetmembersinST_CurrentSkillData _output 0.0))
      (switch Utilities|FlowControl|Switch|SwitchonEN_SkillType (Utilities|GetClassDefaults (.SKill_Class (Utilities|Struct|BreakST_SkillData (.SkillData (Utilities|Struct|BreakST_CurrentSkillData _structout)))))
        (:NewEnumerator1
          _)
        (:NewEnumerator3
          _)
        (:NewEnumerator4
          _)
        (:NewEnumerator6
          _))
      (Game|SpawnActorfromClass (.SKill_Class (Utilities|Struct|BreakST_SkillData (.SkillData (Utilities|Struct|BreakST_CurrentSkillData _structout)))) (Transformation|GetActorTransform _owner) "Undefined" "MultiplyWithRoot" 0 "NewEnumerator0" (.Damage (Utilities|Struct|BreakST_SkillData (.SkillData (Utilities|Struct|BreakST_CurrentSkillData _structout)))) _owner)
      (else
        (Development|PrintString (Utilities|String|Append (.Skill_Name (Utilities|Struct|BreakST_SkillData (.SkillData (Utilities|Struct|BreakST_CurrentSkillData _output)))) " Still Cooltime!") true true "(R=1.000000,G=0.000000,B=0.178356,A=1.000000)" 1.0)))))

(fn AddSkill
  (params (SKillData :type ST%20Skill%20Data%20Structure))
  (bind (_skill_class _skilll_id _skill_name _damage _cooltime _cost) (Utilities|Struct|BreakST_SkillData SKillData))
  (Utilities|Array|AddUnique (Variables|Default|GetSkillList_Entire) (Utilities|Struct|MakeST_CurrentSkillData SKillData _cooltime _cost)))

(fn GetSkillList
  (return (Variables|Default|GetSkillList_Entire)))

(fn FindinSkillList
  (params (SkillData :type ST%20Skill%20Data%20Structure))
  (for (_array_element _array_index) (CallFunction|GetSkillList)
    (if (== (.SKilll_ID (Utilities|Struct|BreakST_SkillData (.SkillData (Utilities|Struct|BreakST_CurrentSkillData _array_element)))) (.SKilll_ID (Utilities|Struct|BreakST_SkillData SkillData)))
      (return _array_index))))

(fn UpdateSkillCooltime
  (params (CurrentSkill :type ST%20Current%20Skill%20Data%20Structure%20%28by%20ref%29))
  (bind (_skilldata _currentcooltime) (Utilities|Struct|BreakST_CurrentSkillData CurrentSkill))
  (Utilities|Struct|SetmembersinST_CurrentSkillData CurrentSkill (+ _currentcooltime (Utilities|Time|GetWorldDeltaSeconds)))
  (if (>= _currentcooltime (.cooltime _skilldata))
    (Default|CallEventDispatcherReadytoSkill CurrentSkill)))

(fn IsReady
  (params (InputPin :type ST%20Current%20Skill%20Data%20Structure%20%28by%20ref%29))
  (bind (_skilldata _currentcooltime) (Utilities|Struct|BreakST_CurrentSkillData InputPin))
  (if (> _currentcooltime (.cooltime _skilldata))
    (return true)
    (else
      (return false))))

(fn UpdateReady
  (params (CurrentSkill :type ST%20Current%20Skill%20Data%20Structure))
  (Development|PrintString (Utilities|String|Append (.skill_name (.SkillData (Utilities|Struct|BreakST_CurrentSkillData CurrentSkill))) " Is Ready") true true "(R=0.000000,G=1.000000,B=0.011662,A=1.000000)"))

(fn ClearSkillList
  (Utilities|Array|Clear (Variables|Default|GetSkillList_Entire)))