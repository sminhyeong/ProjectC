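; BP_DamgeAmount is an actor that shows a floating damage number, then removes itself.
; On BeginPlay it passes its DamageAmount to the Damage_Widget held by its widget component.
; A timeline then lerps the actor 50 units upward from its start location and destroys it when finished.
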(event EventBeginPlay
  (bind _asdamage_widget (Utilities|Casting|CastToDamage_Widget (UserInterface|GetWidget (Variables|Default|GetWidget))))
  (Variables|/Game/SWS/Skill/DamageWidgets/Damage_Widget.Damage_Widget_C|SetDamageAmount _asdamage_widget (Variables|Default|GetDamage%20Amount))
  (bind _output_get (Variables|Default|SetStartLoc (Transformation|GetActorLocation)))
  (Variables|Default|SetEndLoc (+ _output_get "0.000000,0.000000,50.000000"))
  (bind _move_track (Timeline|Timeline%20Move Play)
    (:Update
      (Transformation|SetActorLocation (Math|Vector|Lerp(Vector) (Variables|Default|GetStartLoc) (Variables|Default|GetEndLoc) _move_track) false false))
    (:Finished
      (Actor|DestroyActor))))

(fn ConstructionScript)