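; BP_Skill_BaseClass is a base Blueprint for skills that carries a skill type and its data.
; On BeginPlay it caches the DT_Skill row matching SkillName in CurrentSkillData, then prints the type as debug text if its instigator is a Character.
; GetSkillData performs the table lookup, and GetType exposes SkillType.
; A debug print of the row's fields is left unconnected.
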(event EventBeginPlay
  (Variables|Skill|SetCurrentSkillData (CallFunction|GetSkillData))
  (Utilities|Casting|CastToCharacter (Game|GetInstigator))
  (Development|PrintString (Utilities|String|Append "TYPE " (Utilities|String|EnumtoString (Variables|Skill|GetSkillType)))))

(fn ConstructionScript)

(fn GetSkillData
  (bind _returnvalue (Utilities|GetDataTableRow "/Game/SWS/Skill/DT_Skill.DT_Skill" (Variables|Skill|GetSkill%20Name))
    (:then
      (return _returnvalue))))

(fn GetType
  (return (Variables|Skill|GetSkillType)))