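; Chase skill actor that fires a grab sphere forward from its Instigator and pulls the Instigator to the first other Character it hits.
; A Timeline lerps the sphere toward a point ahead; on overlap the sphere attaches to that victim and stops colliding.
; The Timeline then restarts to lerp the Instigator toward the victim's live location.
; The actor destroys itself when close, when the Timeline finishes, or when its short lifespan expires.
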(event OnComponentBeginOverlap(Sphere)
  (params (OverlappedComponent :type Primitive%20Component%20Object%20Reference) (OtherActor :type Actor%20Object%20Reference) (OtherComp :type Primitive%20Component%20Object%20Reference) (OtherBodyIndex :type Integer) (bFromSweep :type Boolean) (SweepResult :type Hit%20Result%20Structure%20%28by%20ref%29))
  (Utilities|IsValid OtherActor
    (:Is%20Valid
      (bind _ascharacter (Utilities|Casting|CastToCharacter OtherActor))
      (if (!= OtherActor (Variables|Default|GetInstigator))
        (bind _output_get (Variables|Default|SetVictim _ascharacter))
        (Variables|Default|SetIsGrabbing true)
        (Transformation|AttachComponentToComponent (Variables|Default|GetSphere) (Variables|/Script/Engine.Character|GetCapsuleComponent _output_get) "None" "KeepWorld" "KeepWorld" "KeepWorld" true)
        (Collision|SetCollisionEnabled (Variables|Default|GetSphere) "NoCollision")))))

(event EventBeginPlay
  (bind _returnvalue (Transformation|GetActorLocation))
  (|CallParentFunction)
  (Variables|Default|SetStartLoc _returnvalue)
  (Variables|Default|SetEndtLoc (+ _returnvalue (* (Transformation|GetActorForwardVector) 1e+03)))
  (Actor|SetLifeSpan 3.0))

(event EventTick
  (params (DeltaSeconds :type Float%20%28single-precision%29))
  (bind _instigator (Variables|Default|GetInstigator))
  (bind _returnvalue (Transformation|GetActorLocation _instigator))
  (Variables|Default|SetElapsedTime (+ (Variables|Default|GetElapsedTime) DeltaSeconds))
  (bind _newtrack_0 (Timeline|Timeline Play)
    (:Update
      (if (Variables|Default|GetIsGrabbing)
        (Utilities|FlowControl|Sequence
          (:then_0
            (Variables|Default|SetIsGrabbing false)
            (Timeline|Timeline PlayFromStart))
          (:then_1
            (Transformation|SetActorLocation (Variables|Default|GetInstigator) (Math|Vector|Lerp(Vector) (Transformation|GetActorLocation (Variables|Default|GetInstigator)) (Variables|Default|GetEndtLoc) _newtrack_0) false false)))
        (else
          (bind _victim (Variables|Default|GetVictim)
            (:then
              (Variables|Default|SetEndtLoc (Transformation|GetActorLocation _victim))
              (if (< (Math|Vector|Distance(Vector) _returnvalue (Transformation|GetActorLocation _victim)) 1.5e+02)
                (Actor|DestroyActor)
                (else
                  (Transformation|SetActorLocation _instigator (Math|Vector|Lerp(Vector) _returnvalue (Variables|Default|GetEndtLoc) _newtrack_0) false false))))
            (:else
              (Transformation|SetWorldLocation (Variables|Default|GetSphere) (Math|Vector|Lerp(Vector) _returnvalue (Variables|Default|GetEndtLoc) _newtrack_0) false false))))))
    (:Finished
      (Actor|DestroyActor))))

(fn ConstructionScript
  (|CallParentFunction))