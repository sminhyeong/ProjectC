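; BP_Skill_FIreBall is a fireball projectile skill that damages actors it overlaps.
; The construction script sets its skill type, which it prints on BeginPlay alongside a one-second lifespan.
; Tick pushes it forward by a fixed local offset each frame, without sweep or delta-time scaling.
; Sphere overlaps apply damage only on the authority, and the actor persists after a hit until its lifespan ends.
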(event OnComponentBeginOverlap(Sphere)
  (params (OverlappedComponent :type Primitive%20Component%20Object%20Reference) (OtherActor :type Actor%20Object%20Reference) (OtherComp :type Primitive%20Component%20Object%20Reference) (OtherBodyIndex :type Integer) (bFromSweep :type Boolean) (SweepResult :type Hit%20Result%20Structure%20%28by%20ref%29))
  (Networking|SwitchHasAuthority
    (:Authority
      (Game|Damage|ApplyDamage OtherActor (Variables|Default|GetDamage) 0 0))))

(event EventBeginPlay
  (|CallParentFunction)
  (Actor|SetLifeSpan 1.0)
  (Development|PrintString (Utilities|String|Append "TYPE " (Utilities|String|EnumtoString (Variables|Default|GetSkillType)))))

(event EventTick
  (params (DeltaSeconds :type Float%20%28single-precision%29))
  (Transformation|AddActorLocalOffset "10.000000,0.000000,0.000000" false false))

(fn ConstructionScript
  (|CallParentFunction)
  (Variables|Default|SetSkillType "NewEnumerator4"))