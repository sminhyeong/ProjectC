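; Grab skill actor that fires a sphere forward to hook a character other than its instigator and pull it toward the caster.
; A timeline lerps the sphere between start and end points.
; Overlap attaches the victim, disables sphere collision and restarts the timeline toward the instigator's current location.
; The victim detaches only when those endpoints nearly coincide; the actor expires after a short lifespan or when the timeline finishes.
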(event OnComponentBeginOverlap(Sphere)
  (params (OverlappedComponent :type Primitive%20Component%20Object%20Reference) (OtherActor :type Actor%20Object%20Reference) (OtherComp :type Primitive%20Component%20Object%20Reference) (OtherBodyIndex :type Integer) (bFromSweep :type Boolean) (SweepResult :type Hit%20Result%20Structure%20%28by%20ref%29))
  (Utilities|IsValid OtherActor
    (:Is%20Valid
      (bind _ascharacter (Utilities|Casting|CastToCharacter OtherActor))
      (if (!= OtherActor (Variables|Default|GetInstigator))
        (bind _output_get (Variables|Default|SetVictim _ascharacter))
        (Variables|Default|SetIsGrabbing true)
        (Variables|Default|SetStartLoc (Transformation|GetWorldLocation (Variables|Default|GetSphere)))
        (Variables|Default|SetEndtLoc (Transformation|GetActorLocation))
        (bind _ascharacter_2 (Utilities|Casting|CastToCharacter _output_get))
        (Physics|SetSimulatePhysics (Variables|/Script/Engine.Character|GetCapsuleComponent _ascharacter_2) false)
        (Transformation|AttachComponentToComponent _output_get (Variables|Default|GetSphere) "None" "KeepWorld" "KeepWorld" "KeepWorld" true)
        (Collision|SetCollisionEnabled (Variables|Default|GetSphere) "NoCollision")))))

(event EventBeginPlay
  (bind _returnvalue (Transformation|GetActorLocation))
  (|CallParentFunction)
  (Variables|Default|SetStartLoc _returnvalue)
  (Variables|Default|SetEndtLoc (+ _returnvalue (* (Transformation|GetActorForwardVector) 1e+03)))
  (Actor|SetLifeSpan 1.0))

(event EventTick
  (params (DeltaSeconds :type Float%20%28single-precision%29))
  (bind _victim (Variables|Default|GetVictim))
  (bind _newtrack_0 (Timeline|Timeline Play)
    (:Update
      (if (Variables|Default|GetIsGrabbing)
        (Variables|Default|SetIsGrabbing false)
        (Timeline|Timeline PlayFromStart)
        (else
          (Variables|Default|GetVictim
            (:then
              (Variables|Default|SetEndtLoc (Transformation|GetActorLocation (Game|GetInstigator))))
            (:else
              _))
          (Transformation|SetWorldLocation (Variables|Default|GetSphere) (Math|Vector|Lerp(Vector) (Variables|Default|GetStartLoc) (Variables|Default|GetEndtLoc) _newtrack_0) false false)
          (if (Utilities|Operators|EqualEqual (Variables|Default|GetStartLoc) (Variables|Default|GetEndtLoc) 0.1)
            (bind _ascharacter (Utilities|Casting|CastToCharacter _victim))
            (Physics|SetSimulatePhysics (Variables|/Script/Engine.Character|GetCapsuleComponent _ascharacter) true)
            (Transformation|DetachFromActor _victim "KeepWorld" "KeepWorld" "KeepWorld")))))
    (:Finished
      (Actor|DestroyActor))))

(fn ConstructionScript
  (|CallParentFunction))