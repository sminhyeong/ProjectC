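; BP_Skill_Heal is a skill actor that heals players within its sphere when it spawns.
; On BeginPlay it lowers Sphere1, runs the parent logic, then does a one-shot component overlap query.
; Each overlapping BP_Player receives EventHeal with the Damage value as the amount, and the actor's short lifespan is set only on such a hit.
; The construction script sets its SkillType.
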(event EventBeginPlay
  (Transformation|AddWorldOffset (Variables|Default|GetSphere1) "0.000000,0.000000,-90.000000" false false)
  (|CallParentFunction)
  (bind _outactors (Collision|ComponentOverlapActors (Variables|Default|GetSphere1) (Math|Transform|MakeTransform "0, 0, 0" "0, 0, 0" "1.000000,1.000000,1.000000") (Utilities|Array|MakeArray "ObjectTypeQuery8" "ObjectTypeQuery3" "ObjectTypeQuery4") 0))
  (for _array_element _outactors
    (bind _asbp_player (Utilities|Casting|CastToBP_Player _array_element))
    (Default|EventHeal _asbp_player (Variables|Default|GetDamage))
    (Actor|SetLifeSpan 2.0)))

(fn ConstructionScript
  (|CallParentFunction)
  (Variables|Default|SetSkillType "NewEnumerator6"))