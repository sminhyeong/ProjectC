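; Wrecking Ball skill actor that knocks back characters touching its sphere.
; On BeginPlay it snaps onto its instigator, takes its lifespan from the skill data's Duration and plays a heavy attack startup montage.
; On authority, each new sphere overlap loops over the overlapping actors and launches Characters away from the actor through a Req/Res knockback event pair.
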(event OnComponentBeginOverlap(Sphere)
  (params (OverlappedComponent :type Primitive%20Component%20Object%20Reference) (OtherActor :type Actor%20Object%20Reference) (OtherComp :type Primitive%20Component%20Object%20Reference) (OtherBodyIndex :type Integer) (bFromSweep :type Boolean) (SweepResult :type Hit%20Result%20Structure%20%28by%20ref%29))
  (Networking|SwitchHasAuthority
    (:Authority
      (for _array_element (Collision|GetOverlappingActors (Variables|Default|GetSphere) 0 :!class /Script/Engine.PrimitiveComponent)
        (bind _ascharacter (Utilities|Casting|CastToCharacter _array_element))
        (CallFunction|ReqKnockback _ascharacter)))))

(event Custom|ReqKnockback
  (params (Target :type Character%20Object%20Reference))
  (CallFunction|ReSKnockback Target))

(event Custom|ResKnockback
  (params (Target :type Character%20Object%20Reference))
  (Character|LaunchCharacter Target (* (Math|Vector|Normalize (- (Transformation|GetActorLocation Target) (Transformation|GetActorLocation))) 1e+03) false false))

(event EventBeginPlay
  (|CallParentFunction)
  (Transformation|AttachActorToActor (Variables|Default|GetInstigator) "None" "SnapToTarget" "SnapToTarget" "SnapToTarget" true)
  (Actor|SetLifeSpan (.Duration (Utilities|Struct|BreakST_SkillData (CallFunction|GetSkillData))))
  (bind _ascharacter (Utilities|Casting|CastToCharacter (Game|GetInstigator)))
  (Animation|PlayAnimMontage _ascharacter "/Game/KJK/GM/AnimTest/anim_attack_heavy_startup_Montage.anim_attack_heavy_startup_Montage" 1.0 "None"))

(event EventTick
  (params (DeltaSeconds :type Float%20%28single-precision%29)))

(fn ConstructionScript
  (|CallParentFunction))