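; BP_DungeonToLobbyPotal is a portal actor that opens a back-to-lobby UI when a character enters it.
; Its Box begin-overlap runs only with authority, filters for any Character and prints a debug message.
; It then creates BackLobbyWidget for player controller 0, adds it to the viewport and enables Game-and-UI input with the mouse cursor, regardless of which character overlapped.
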(event OnComponentBeginOverlap(Box)
  (params (OverlappedComponent :type Primitive%20Component%20Object%20Reference) (OtherActor :type Actor%20Object%20Reference) (OtherComp :type Primitive%20Component%20Object%20Reference) (OtherBodyIndex :type Integer) (bFromSweep :type Boolean) (SweepResult :type Hit%20Result%20Structure%20%28by%20ref%29))
  (bind _returnvalue (Game|GetPlayerController 0))
  (Networking|SwitchHasAuthority
    (:Authority
      (Utilities|Casting|CastToCharacter OtherActor)
      (Development|PrintString (Utilities|String|Append (Utilities|GetDisplayName OtherActor) " : OverlapToPotal"))
      ;[0.15 0.15 0.15 0.5] widget
      (bind _returnvalue_2 (UserInterface|CreateWidget "/Game/YSJ/Widgets/BackLobbyWidget.BackLobbyWidget_C" _returnvalue))
      (bind _output_get (Variables|Default|SetBackLobbyWidget _returnvalue_2))
      (UserInterface|Viewport|AddtoViewport _output_get 0)
      (Input|SetInputModeGameandUI _returnvalue 0 "DoNotLock" true false)
      (Variables|/Script/Engine.PlayerController|SetbShowMouseCursor _returnvalue true))))

(event EventBeginPlay)

(event Collision|EventActorBeginOverlap
  (params (OtherActor :type Actor%20Object%20Reference)))

(event EventTick
  (params (DeltaSeconds :type Float%20%28single-precision%29)))

(fn ConstructionScript)