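; Game state that handles connection feedback, map-loading UI and the reward step after a monster death request.
; Connection state changes recolor the status indicators on the login and server list widgets.
; A map-loading response shows a wait message, switches to UI-only input with cursor and collapses dungeon portal entry widgets.
; A monster death request turns every Monster spawner into a Chest spawner, spawns it and triggers all dungeon portal spawners.
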(event Custom|MapLoadingRes
  (params (LoadingText :type String))
  (bind _returnvalue (Game|GetPlayerController 0))
  (bind _returnvalue_2 (Game|GetPlayerController 0))
  (Development|PrintString (Utilities|String|Append "Map Loading Res Controller : " (Utilities|GetDisplayName _returnvalue_2)) true true "(R=0.000000,G=0.660000,B=1.000000,A=1.000000)" 1e+01)
  (bind _returnvalue_3 (UserInterface|CreateWidget "/Game/YSJ/Widgets/WaitPlzWidget.WaitPlzWidget_C" _returnvalue_2))
  (Rendering|Components|TextRender|SetText (Variables|/Game/YSJ/Widgets/WaitPlzWidget.WaitPlzWidget_C|GetMessage _returnvalue_3) (Utilities|Text|ToText(String) LoadingText))
  (UserInterface|Viewport|AddtoViewport _returnvalue_3 0)
  (Input|SetInputModeUIOnly _returnvalue 0 "DoNotLock" false)
  (Variables|/Script/Engine.PlayerController|SetbShowMouseCursor _returnvalue true)
  (bind _outactors (Actor|GetAllActorsOfClass "/Game/YSJ/BP_DungeonPotal.BP_DungeonPotal_C"))
  (for _array_element _outactors
    (bind _enterdungeonwidget (Variables|/Game/YSJ/BP_DungeonPotal.BP_DungeonPotal_C|GetEnterDungeonWidget _array_element)
      (:then
        (Widget|SetVisibility _enterdungeonwidget "Collapsed"))
      (:else))))

(event Custom|MonsterDeathReq
  (bind _outactors (Actor|GetAllActorsOfClass "/Game/KHC/Item/BP_ObjectSpawner.BP_ObjectSpawner_C"))
  (for _array_element _outactors
    (Utilities|IsValid (Actor|GetComponentbyClass _array_element "/Script/ProjectC.ObjectSpawnComponent")
      (:Is%20Valid
        (switch Utilities|FlowControl|Switch|SwitchonESpawnObjectType (Variables|/Script/ProjectC.ObjectSpawnComponent|GetSpawnObjectType (Actor|GetComponentbyClass _array_element "/Script/ProjectC.ObjectSpawnComponent"))
          (:Monster
            (Variables|/Script/ProjectC.ObjectSpawnComponent|SetSpawnObjectType (Actor|GetComponentbyClass _array_element "/Script/ProjectC.ObjectSpawnComponent") "Chest")
            (Class|ObjectSpawnComponent|SpawnObjectat (Actor|GetComponentbyClass _array_element "/Script/ProjectC.ObjectSpawnComponent"))
            (bind _outactors_2 (Actor|GetAllActorsOfClass "/Game/KHC/Item/BP_DungeonPortalSpawner.BP_DungeonPortalSpawner_C"))
            (for _array_element_2 _outactors_2
              (Default|SpawnPortal _array_element_2))))))))

(event EventBeginPlay)

(fn ConstructionScript)

(fn BPGameStartGameStateAutoGenFunc
  (params (NewState :type ENetConnectionState%20Enum :default "Disconnected"))
  (switch Utilities|FlowControl|Switch|SwitchonENetConnectionState NewState
    (:Disconnected
      (Default|ShowConnetState (Variables|Default|GetLoginWidget) "(R=1.000000,G=0.000000,B=0.019608,A=1.000000)")
      (Default|ShowConnectState (Variables|Default|GetServerListWIdget) "(R=1.000000,G=0.000000,B=0.019608,A=1.000000)"))
    (:Connecting
      (Default|ShowConnetState (Variables|Default|GetLoginWidget) "(R=0.149020,G=1.000000,B=0.054902,A=1.000000)" :!label _label)
      (Default|ShowConnectState (Variables|Default|GetServerListWIdget) "(R=0.149020,G=1.000000,B=0.054902,A=1.000000)"))
    (:Connected
      (Default|ShowConnetState (Variables|Default|GetLoginWidget) "(R=0.000000,G=0.044782,B=1.000000,A=1.000000)")
      (Default|ShowConnectState (Variables|Default|GetServerListWIdget) "(R=0.000000,G=0.043137,B=1.000000,A=1.000000)"))
    (:Reconnecting
      (goto _label))
    (:Failed
      (Default|ShowConnetState (Variables|Default|GetLoginWidget))
      (Default|ShowConnectState (Variables|Default|GetServerListWIdget)))))